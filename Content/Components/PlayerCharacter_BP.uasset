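; Player character Blueprint that handles the toolbar and equipment UI, nine-slot mouse-wheel item selection, a point light held above the player and saving.
; E toggles the equipment screen with cursor and input mode, while F1 toggles the toolbar.
; P saves player transform, flattened inventory structs and compressed world to slots under the world name.
; LoadPlayer rebuilds items and spawns a platform beneath the restored position; LoadWorld is disconnected.
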(event EventBeginPlay
  (bind _returnvalue (UserInterface|CreateWidget "/Game/Components/UI/ToolBar_BP.ToolBar_BP_C" (Game|GetPlayerController 0)))
  (bind _output_get (Variables|Default|SetToolBar _returnvalue))
  (UserInterface|Viewport|AddtoViewport _output_get 0)
  (bind _returnvalue_2 (SaveGame|CreateSaveGameObject "/Game/SaveStructs/savePlayer.savePlayer_C"))
  (Variables|Default|SetsaveInstance _returnvalue_2))

(event Collision|EventActorBeginOverlap
  (params (OtherActor :type Actor%20Object%20Reference)))

(event EventTick
  (params (DeltaSeconds :type Float%20%28single-precision%29))
  (bind _returnvalue (Transformation|GetActorLocation))
  (Transformation|SetWorldLocation (Variables|Default|GetPointLight) (Math|Vector|MakeVector (.x _returnvalue) (.y _returnvalue) (+ (.z _returnvalue) 1e+02)) false false))

(event Input|KeyboardEvents|E
  (params (Key :type Key%20Structure :default "None"))
  (bind _returnvalue (Game|GetPlayerController 0))
  (bind _currentlyopenuis (Variables|Default|GetcurrentlyOpenUIs))
  (:Pressed
    (if (not (Variables|Default|GetisGuiOpen))
      (bind _returnvalue_2 (UserInterface|CreateWidget "/Game/Components/UI/Equipment_BP.Equipment_BP_C" _returnvalue))
      (bind _output_get (Variables|Default|Setequipment _returnvalue_2))
      (UserInterface|Viewport|AddtoViewport _output_get 0)
      (Utilities|Array|Add (Variables|Default|GetcurrentlyOpenUIs) _output_get)
      (bind _returnvalue_3 (UserInterface|CreateWidget "/Game/Components/UI/ItemStatsShow.ItemStatsShow_C" _returnvalue))
      (Variables|Default|SetItemStatsShow _returnvalue_3)
      (Variables|/Script/Engine.PlayerController|SetbShowMouseCursor _returnvalue true)
      (Variables|Default|SetisGuiOpen true)
      (Input|SetInputModeGameandUI _returnvalue (Variables|Default|Getequipment) "LockAlways" true)
      (Variables|Default|SetshowItemStats true)
      (else
        (for _array_element _currentlyopenuis
          (Widget|RemovefromParent _array_element))
        (Utilities|Array|Clear _currentlyopenuis)
        (Widget|RemovefromParent (Variables|Default|GetItemStatsShow))
        (Variables|/Script/Engine.PlayerController|SetbShowMouseCursor _returnvalue false)
        (Variables|Default|SetisGuiOpen false)
        (Input|SetInputModeGameOnly _returnvalue)
        (Variables|Default|SetisItemDraggableGuiOpen false)))))

(event Input|KeyboardEvents|F1
  (params (Key :type Key%20Structure :default "None"))
  (:Pressed
    (Utilities|FlowControl|FlipFlop
      (:A
        (Widget|RemovefromParent (Variables|Default|GetToolBar)))
      (:B
        (UserInterface|Viewport|AddtoViewport (Variables|Default|GetToolBar) 0)))))

(event Input|MouseEvents|MouseWheelUp
  (params (Key :type Key%20Structure :default "None"))
  (:Pressed
    (Default|BringBackUnselectedItemFrame (Variables|Default|GetToolBar))
    (bind _output_get (Variables|Default|SetselectedItem (+ (Variables|Default|GetselectedItem) 1)))
    (if (> _output_get 8)
      (Variables|Default|SetselectedItem 0))
    (Default|ChangeSelectedItemPosition (Variables|Default|GetToolBar))))

(event Input|MouseEvents|MouseWheelDown
  (params (Key :type Key%20Structure :default "None"))
  (:Pressed
    (Default|BringBackUnselectedItemFrame (Variables|Default|GetToolBar))
    (bind _output_get (Variables|Default|SetselectedItem (- (Variables|Default|GetselectedItem) 1)))
    (if (< _output_get 0)
      (Variables|Default|SetselectedItem 8))
    (Default|ChangeSelectedItemPosition (Variables|Default|GetToolBar))))

(event Input|KeyboardEvents|P
  (params (Key :type Key%20Structure :default "None"))
  (:Pressed
    (CallFunction|SavePlayer)
    (CallFunction|SaveWorld)))

(event Input|KeyboardEvents|O
  (params (Key :type Key%20Structure :default "None")))

(event Input|KeyboardEvents|G
  (params (Key :type Key%20Structure :default "None")))

(event Input|KeyboardEvents|H
  (params (Key :type Key%20Structure :default "None")))

(event Input|KeyboardEvents|Escape
  (params (Key :type Key%20Structure :default "None")))

(fn ConstructionScript)

(fn SetEquipmentSave
  (params (Save%20Instance :type Save%20Player%20Object%20Reference))
  (bind _itemsinequipment (Variables|/Game/SaveStructs/savePlayer.savePlayer_C|GetitemsInEquipment Save%20Instance))
  (for _array_element (Variables|Default|GetitemsInEquipment)
    (bind _asstackable_item (Utilities|Casting|CastToStackableItem _array_element)
      (:then
        (Utilities|Array|Add _itemsinequipment (Utilities|Struct|MakeItem (Variables|/Script/Caves_Taint.Item|GetitemName _array_element) (Variables|/Script/Caves_Taint.Item|GetplacedItemClass _array_element) (Variables|/Script/Caves_Taint.Item|Getstackable _array_element) (Variables|/Script/Caves_Taint.StackableItem|Getstack _asstackable_item))))
      (:CastFailed
        (Utilities|Array|Add _itemsinequipment (Utilities|Struct|MakeItem (Variables|/Script/Caves_Taint.Item|GetitemName _array_element) (Variables|/Script/Caves_Taint.Item|GetplacedItemClass _array_element) (Variables|/Script/Caves_Taint.Item|Getstackable _array_element) 0))))))

(fn LoadEquipmentSaveStruct
  (params (NewParam :type Save%20Player%20Object%20Reference))
  (bind _self self)
  (bind _itemsinequipment (Variables|Default|GetitemsInEquipment))
  (Utilities|Array|Clear (Variables|Default|GetitemsInEquipment))
  (for (_array_element _array_index) (Variables|/Game/SaveStructs/savePlayer.savePlayer_C|GetitemsInEquipment NewParam)
    (if (.stackable _array_element)
      (bind _returnvalue (Game|ConstructObjectfromClass "/Script/Caves_Taint.StackableItem" _self))
      (Variables|/Script/Caves_Taint.Item|SetitemName _returnvalue (.itemname _array_element))
      (Variables|/Script/Caves_Taint.Item|SetplacedItemClass _returnvalue (.placeditemclass _array_element))
      (Variables|/Script/Caves_Taint.Item|Setstackable _returnvalue true)
      (Variables|/Script/Caves_Taint.StackableItem|Setstack _returnvalue (.stack _array_element))
      (Variables|/Script/Caves_Taint.Item|SetequipmentIndex _returnvalue 0)
      (Utilities|Array|Add _itemsinequipment _returnvalue)
      (else
        (bind _returnvalue_2 (Game|ConstructObjectfromClass "/Script/Caves_Taint.Item" _self))
        (Variables|/Script/Caves_Taint.Item|SetitemName _returnvalue_2 (.itemname _array_element))
        (Variables|/Script/Caves_Taint.Item|SetplacedItemClass _returnvalue_2 (.placeditemclass _array_element))
        (Variables|/Script/Caves_Taint.Item|Setstackable _returnvalue_2 false)
        (Variables|/Script/Caves_Taint.Item|SetequipmentIndex _returnvalue_2 _array_index)
        (Utilities|Array|Add _itemsinequipment _returnvalue_2))))
  (Class|PlayerCharacter|UpdateItemIndexes))

(fn OnWorldLoaded
  (params (NewParam :type World%20Object%20Reference)))

(fn SaveWorld
  (bind _outsave (Class|VoxelDataTools|GetCompressedSave (Variables|Default|GetworldReference)))
  (bind _returnvalue (SaveGame|CreateSaveGameObject "/Game/SaveStructs/saveWorld.saveWorld_C"))
  (Variables|/Game/SaveStructs/saveWorld.saveWorld_C|SetworldStruct _returnvalue _outsave)
  (SaveGame|SaveGametoSlot _returnvalue (Utilities|String|Append (Variables|Default|GetcurrentWorldName) "/world")))

(fn LoadWorld)

(fn LoadPlayerParams
  (params (savePlayer :type Save%20Player%20Object%20Reference))
  (bind _playerposition (Variables|/Game/SaveStructs/savePlayer.savePlayer_C|GetplayerPosition savePlayer))
  (Game|SpawnActorfromClass "/Game/SaveStructs/spawnPlatform.spawnPlatform_C" (Math|Transform|MakeTransform (Math|Vector|MakeVector (.x _playerposition) (.y _playerposition) (- (.z _playerposition) 5e+01)) "0, 0, 0" "1,1,1") "Undefined" 0 0)
  (Transformation|SetActorLocation (Math|Vector|MakeVector (.x _playerposition) (.y _playerposition) (.z _playerposition)) false false)
  (Transformation|SetActorRotation (Variables|/Game/SaveStructs/savePlayer.savePlayer_C|GetplayerRotation savePlayer)))

(fn LoadPlayer
  (bind _returnvalue (SaveGame|LoadGamefromSlot (Utilities|String|Append (Variables|Default|GetcurrentWorldName) "/player")))
  (bind _assave_player (Utilities|Casting|CastTosavePlayer _returnvalue))
  (CallFunction|LoadPlayerParams _assave_player)
  (CallFunction|LoadEquipmentSaveStruct _assave_player))

(fn SetPlayerParamsSave
  (params (save%20instance :type Save%20Player%20Object%20Reference))
  (Variables|/Game/SaveStructs/savePlayer.savePlayer_C|SetplayerPosition save%20instance (Transformation|GetActorLocation))
  (Variables|/Game/SaveStructs/savePlayer.savePlayer_C|SetplayerRotation save%20instance (Transformation|GetActorRotation)))

(fn SavePlayer
  (bind _returnvalue (SaveGame|CreateSaveGameObject "/Game/SaveStructs/savePlayer.savePlayer_C"))
  (CallFunction|SetEquipmentSave _returnvalue)
  (CallFunction|SetPlayerParamsSave _returnvalue)
  (SaveGame|SaveGametoSlot _returnvalue (Utilities|String|Append (Variables|Default|GetcurrentWorldName) "/player")))